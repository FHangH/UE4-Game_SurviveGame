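; Game mode for a survival game that handles game over, replay, quit and the longest-survival record.
; On BeginPlay it caches the game instance, global timer and warehouse, then creates the main UI.
; Game over stops the timer and shows the finished screen with time survived and a record message.
; CheckSurvivalTime compares against a SaveGame slot, saving new records with an offset day, though the comparison uses the raw day.
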(event `self.ReceiveBeginPlay`
  (`|ExecutionSequence`
    (:`then_0`
      (set `self.MyGameInstance` (cast `/Game/MyDemo/Blueprints/Object/BPGameIns_MyInstance` (`GameplayStatics.GetGameInstance`) :!pure true)))
    (:`then_1`
      (bind _outactors (`GameplayStatics.GetAllActorsOfClass` "/Game/MyDemo/Blueprints/Object/Actor/BPActor_GlobalSetTimer.BPActor_GlobalSetTimer_C"))
      (set `self.GlobalSetTimer` (`|GetArrayItem` _outactors))
      (`/Game/MyDemo/Blueprints/Object/BPGameIns_MyInstance.CreateMainUI` (`self.MyGameInstance`)))
    (:`then_2`
      (bind _outactors_2 (`GameplayStatics.GetAllActorsOfClass` "/Game/MyDemo/Blueprints/Object/Actor/BPA_Warehouse.BPA_Warehouse_C"))
      (set `self.Warehouse` (`|GetArrayItem` _outactors_2)))))

(event `GameOverInfoTip`
  (bind _globalsettimer (`self.GlobalSetTimer`))
  (bind _mygameinstance (`self.MyGameInstance`))
  (bind _curday (`/Game/MyDemo/Blueprints/Object/Actor/BPActor_GlobalSetTimer.CurDay` _globalsettimer))
  (bind _curhour (`/Game/MyDemo/Blueprints/Object/Actor/BPActor_GlobalSetTimer.CurHour` _globalsettimer))
  (`/Game/MyDemo/Blueprints/Object/Actor/BPActor_GlobalSetTimer.StopTimer` _globalsettimer)
  (`/Game/MyDemo/Blueprints/Object/BPGameIns_MyInstance.HideAllPanel` _mygameinstance)
  (`/Game/MyDemo/Blueprints/Object/BPGameIns_MyInstance.CreatGameFinished` _mygameinstance)
  (bind _recordtext (`self.Check Survival Time` _curday _curhour))
  (`/Game/MyDemo/Blueprints/UI/UI_GameFinished.SetShowSurivalTimeText` (`/Game/MyDemo/Blueprints/Object/BPGameIns_MyInstance.UI_GameFinished` _mygameinstance) _curday _curhour _recordtext))

(event `ReplayGame`
  (`GameplayStatics.OpenLevel` "MainMap")
  (`WidgetBlueprintLibrary.SetInputMode_GameOnly` (`GameplayStatics.GetPlayerController` 0)))

(event `ExitGame`
  (`KismetSystemLibrary.QuitGame` (`GameplayStatics.GetPlayerController` 0) "Quit"))

(fn `Check Survival Time`
  (params (Day :type Integer) (Hour :type Integer))
  (returns (RecordText :type String))
  (locals (fNewTimeDate :type Integer :default 0) (fNewDay :type Integer) (fNewHour :type Integer))
  (set `local.fNewDay` (- Day 8))
  (set `local.fNewHour` Hour)
  (set `local.fNewTimeDate` (+ (* Day 24) Hour))
  (bind _returnvalue (`GameplayStatics.DoesSaveGameExist` "MaxTime"))
  (if _returnvalue
    (bind _returnvalue_2 (`GameplayStatics.LoadGameFromSlot` "MaxTime"))
    (bind _asbpa_my_save_game (cast `/Game/MyDemo/Blueprints/Object/BPA_MySaveGame` _returnvalue_2))
    (bind _maxday (`/Game/MyDemo/Blueprints/Object/BPA_MySaveGame.MaxDay` _asbpa_my_save_game))
    (bind _maxhour (`/Game/MyDemo/Blueprints/Object/BPA_MySaveGame.MaxHour` _asbpa_my_save_game))
    (bind _returnvalue_3 (- (`local.fNewTimeDate`) (+ (* _maxday 24) _maxhour)))
    (if (> _returnvalue_3 0)
      _
      (else
        (if (== _returnvalue_3 0)
          _
          (else
            _))
        (return (`KismetTextLibrary.Conv_TextToString` (`|FormatText` "Survival Record: Max Record {MaxDay}Day {MaxHour}Hour" _maxday _maxhour))))))
  (bind _returnvalue_4 (`GameplayStatics.CreateSaveGameObject` "/Game/MyDemo/Blueprints/Object/BPA_MySaveGame.BPA_MySaveGame_C"))
  (set `/Game/MyDemo/Blueprints/Object/BPA_MySaveGame.MaxDay` (`local.fNewDay`) _returnvalue_4)
  (set `/Game/MyDemo/Blueprints/Object/BPA_MySaveGame.MaxHour` (`local.fNewHour`) _returnvalue_4)
  (`GameplayStatics.SaveGameToSlot` _returnvalue_4 "MaxTime")
  (return "Survival Record: New Record"))

(fn `UserConstructionScript`)