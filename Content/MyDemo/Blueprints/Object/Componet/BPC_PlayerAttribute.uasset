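; BPC_PlayerAttribute is an actor component that holds the player's health as current and maximum HP.
; On BeginPlay it fills current HP to the maximum and caches its owner cast to SurviveCharacter.
; GetCurHPSacle returns current HP divided by maximum as a health ratio.
; The file contains no damage or healing logic, and Tick is empty.
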(event `self.ReceiveBeginPlay`
  (`self.InitMaxHP`)
  (set `self.PlayerCharacter` (cast `/Game/MyDemo/Blueprints/RoleAndAI/Role/SurviveCharacter` (`self.GetOwner`) :!pure true)))

(event `self.ReceiveTick`
  (params (DeltaSeconds :type "Float (single-precision)")))

(fn `GetCurHPSacle`
  (returns (HPScale :type "Float (double-precision)"))
  (return (/ (`self.CurHP`) (`self.MaxHP`))))

(fn `InitMaxHP`
  (set `self.CurHP` (`self.MaxHP`)))