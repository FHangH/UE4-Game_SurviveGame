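; Game instance that acts as the central manager for the game's UI panels: main HUD, message box, pick table, inventory, warehouse and game-finished screen.
; ShowPanel lazily creates each widget into a by-ref variable, reuses it afterwards and adds it to the viewport.
; An active-panel counter drives input mode: modal panels enable Game and UI with cursor, and hiding the last restores Game Only.
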(event `CreateMainUI`
  (`self.ShowPanel` "/Game/MyDemo/Blueprints/UI/UI_Main.UI_Main_C" (`self.UI_Main`) false)
  (`self.ShowPanel` "/Game/MyDemo/Blueprints/UI/Panel/UI_MessageBoxPanel.UI_MessageBoxPanel_C" (`self.UI_MessagePanel`) false)
  (set `self.ActiveUICount` 0))

(event `PushMessageAtPanel`
  (params (MessageTextContent :type String))
  (`/Game/MyDemo/Blueprints/UI/Panel/UI_MessageBoxPanel.PushMessageAtPanel` (`self.UI_MessagePanel`) MessageTextContent))

(event `CreatePickTablePanel`
  (`self.ShowPanel` "/Game/MyDemo/Blueprints/UI/Panel/UI_PicktablePanel.UI_PicktablePanel_C" (`self.UI_PickTablePanel`)))

(event `RemovePickTablePanel`
  (`self.HideUIPanel` (`self.UI_PickTablePanel`)))

(event `CreateInventory`
  (`self.ShowPanel` "/Game/MyDemo/Blueprints/UI/Panel/UI_InventoryPanel.UI_InventoryPanel_C" (`self.UI_Inventory`)))

(event `RemoveInventory`
  (`self.HideUIPanel` (`self.UI_Inventory`)))

(event `CreateWarehouse`
  (`self.ShowPanel` "/Game/MyDemo/Blueprints/UI/Panel/UI_WarehousePanel.UI_WarehousePanel_C" (`self.UI_Warehouse`)))

(event `RemoveWarehouse`
  (`self.HideUIPanel` (`self.UI_Warehouse`)))

(event `CreatGameFinished`
  (`self.ShowPanel` "/Game/MyDemo/Blueprints/UI/UI_GameFinished.UI_GameFinished_C" (`self.UI_GameFinished`)))

(event `HideAllPanel`
  (`self.HideUIPanel` (`self.UI_PickTablePanel`))
  (`self.HideUIPanel` (`self.UI_Inventory`))
  (`self.HideUIPanel` (`self.UI_Warehouse`)))

(fn `HideUIPanel`
  (params (Panelvariable :type "Widget Object Reference"))
  (bind _returnvalue (`GameplayStatics.GetPlayerController` 0))
  (`/Engine/EditorBlueprintResources/StandardMacros.IsValid` Panelvariable
    (:`Is Valid`
      (if (`Widget.IsVisible` Panelvariable)
        (`Widget.RemoveFromParent` Panelvariable)
        (bind _result (`/Engine/EditorBlueprintResources/StandardMacros.DecrementInt` (`self.ActiveUICount`))
          (:`  `
            (if (== _result 0)
              (`WidgetBlueprintLibrary.SetInputMode_GameOnly` _returnvalue)
              (set `PlayerController.bShowMouseCursor` false _returnvalue)
              (return))))))))

(fn `ShowPanel`
  (params (PanelTypeClass :type "UserWidget Class Reference") (PanelVariable :type "UserWidget Object Reference (by ref)") (IsChangeUIMode :type Boolean :default true))
  (bind _returnvalue (`GameplayStatics.GetPlayerController` 0))
  (`/Engine/EditorBlueprintResources/StandardMacros.IsValid` PanelVariable
    (:`Is Valid`
      (if (not (`Widget.IsInViewport` PanelVariable))
        (`UserWidget.AddToViewport` PanelVariable 0 :!label _label)
        (if IsChangeUIMode
          (`/Engine/EditorBlueprintResources/StandardMacros.IncrementInt` (`self.ActiveUICount`)
            (:`  `
              (`WidgetBlueprintLibrary.SetInputMode_GameAndUIEx` _returnvalue PanelVariable)
              (set `PlayerController.bShowMouseCursor` true _returnvalue))))))
    (:`Is Not Valid`
      (bind _returnvalue_2 (`|CreateWidget` PanelTypeClass (`GameplayStatics.GetPlayerController` 0)))
      (`|VariableSetRef` PanelVariable _returnvalue_2)
      (goto _label))))